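; HitVfx is a short-lived hit effect actor that plays a flipbook sprite and follows its owner.
; On BeginPlay it stores the owner and an offset of owner location minus its own, then destroys itself after one flipbook length.
; Each Tick it moves to the owner's location plus that offset while the owner is valid, which mirrors its spawn position across the owner.
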(event EventBeginPlay
  (bind _output_get (Variables|Default|SetOwnerActor (Components|GetOwner)))
  (Variables|Default|SetActorOffset (- (Transformation|GetActorLocation _output_get) (Transformation|GetActorLocation)))
  (Utilities|FlowControl|Delay (Class|PaperFlipbookComponent|GetFlipbookLength (Variables|Default|GetSprite)))
  (Actor|DestroyActor))

(event EventTick
  (params (DeltaSeconds :type Float%20%28single-precision%29))
  (bind _owneractor (Variables|Default|GetOwnerActor))
  (if (Utilities|IsValid _owneractor)
    (Transformation|SetActorLocation (+ (Transformation|GetActorLocation _owneractor) (Variables|Default|GetActorOffset)) false false)))

(fn ConstructionScript)