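; Base enemy character with health and stability bars, contact damage to the hero, and AI blackboard flags for seeing the hero and being stunned.
; Knockback hits drain stability, and at zero they launch and temporarily stun the enemy.
; Stability refills after a retriggerable delay, and low health marks the enemy grabbable.
; Damage spawns hit VFX at random capsule points, shield contact launches the enemy, and zero health destroys it.
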(event OnComponentHit(CapsuleComponent)
  (params (HitComponent :type Primitive%20Component%20Object%20Reference) (OtherActor :type Actor%20Object%20Reference) (OtherComp :type Primitive%20Component%20Object%20Reference) (NormalImpulse :type Vector :default "0, 0, 0") (Hit :type Hit%20Result%20Structure%20%28by%20ref%29))
  (bind _asmain_hero_char (Utilities|Casting|CastToMainHeroChar OtherActor)
    (:then
      (Game|Damage|ApplyDamage _asmain_hero_char (Variables|Default|GetDefaultDamage) 0 self))
    (:CastFailed
      (Utilities|Casting|CastToShield OtherActor)
      (Components|Movement|StopMovementImmediately (Variables|Character|GetCharacterMovement))
      (Character|LaunchCharacter "100.000000,0.000000,50.000000" false false))))

(event OnSeePawn(PawnSensing)
  (params (Pawn :type Pawn%20Object%20Reference))
  (bind _blackboard (Variables|Default|GetBlackboard))
  (Utilities|Casting|CastToMainHeroChar Pawn)
  (AI|Components|Blackboard|SetValueasBool _blackboard (Utilities|Name|MakeLiteralName "CanSeeHero") true)
  (Utilities|FlowControl|RetriggerableDelay 5.0)
  (AI|Components|Blackboard|SetValueasBool _blackboard (Utilities|Name|MakeLiteralName "CanSeeHero") false))

(event Custom|OnDamageTaken
  (params (Damage :type Float%20%28double-precision%29))
  (CallFunction|CheckStun)
  (bind _output_get (Variables|Default|SetHealth (- (Variables|Default|GetHealth) Damage)))
  (if (<= _output_get 0.0)
    (CallFunction|Kill)
    (else
      (CallFunction|CheckGrab)
      (CallFunction|SetBars)
      (CallFunction|OnDamageEnd)
      (if (Variables|Default|GetIsStunned)
        (Utilities|FlowControl|RetriggerableDelay (Variables|Default|GetStunDuration))
        (Variables|Default|SetIsStunned false)
        (AI|Components|Blackboard|SetValueasBool (Variables|Default|GetBlackboard) (Utilities|Name|MakeLiteralName "IsStunned") false)))))

(event Custom|OnStabilityRestore
  (Variables|Default|SetStability (Variables|Default|GetMaxStability))
  (CallFunction|SetStabilityBar))

(event Custom|OnDamageEnd
  (Utilities|FlowControl|RetriggerableDelay (Variables|Default|GetStabilityTimer))
  (CallFunction|OnStabilityRestore))

(event EventBeginPlay
  (bind _asenemy_bars (Utilities|Casting|CastToEnemyBars (UserInterface|GetUserWidgetObject (Variables|Default|GetWidget))))
  (Variables|Default|SetBars _asenemy_bars)
  (Variables|/Script/Engine.CharacterMovementComponent|SetMaxWalkSpeed (Variables|Character|GetCharacterMovement) 1e+02)
  (Variables|Default|SetDefaultDamage 1e+01)
  (Variables|Default|SetBlackboard (AI|GetBlackboard (AI|GetAIController self))))

(event Collision|EventActorBeginOverlap
  (params (OtherActor :type Actor%20Object%20Reference)))

(event EventTick
  (params (DeltaSeconds :type Float%20%28single-precision%29)))

(event Game|Damage|EventAnyDamage
  (params (Damage :type Float%20%28single-precision%29) (DamageType :type Damage%20Type%20Object%20Reference) (InstigatedBy :type Controller%20Object%20Reference) (DamageCauser :type Actor%20Object%20Reference))
  (bind _canbedamaged (CallFunction|CanbeDamaged))
  (if _canbedamaged
    (CallFunction|OnDamageTaken Damage)
    (CallFunction|SpawnHitVfx)))

(fn ConstructionScript)

(fn CanbeDamaged
  (return (not (Variables|Default|GetIsImmune))))

(fn ApplyDamagewithKnockback
  (params (Damage :type Float%20%28double-precision%29) (Dealer :type Actor%20Object%20Reference) (Knockback :type Vector))
  (bind _output_get (Variables|Default|SetStability (- (Variables|Default|GetStability) (* (Variables|Default|GetMaxStability) (Variables|Default|GetStabilityDamage)))))
  (Game|Damage|ApplyDamage self Damage 0 Dealer)
  (if (<= _output_get 0.0)
    (if (Utilities|IsValid self)
      (Components|Movement|StopMovementImmediately (Variables|Character|GetCharacterMovement))
      (Character|LaunchCharacter Knockback false false))))

(fn SetHealthbar
  (Variables|/Game/Blueprints/Enemies/EnemyBars.EnemyBars_C|SetHealth (Variables|Default|GetBars) (/ (Variables|Default|GetHealth) (Variables|Default|GetMaxHealth))))

(fn SetStabilityBar
  (Variables|/Game/Blueprints/Enemies/EnemyBars.EnemyBars_C|SetStability (Variables|Default|GetBars) (/ (Variables|Default|GetStability) (Variables|Default|GetMaxStability))))

(fn SetBars
  (CallFunction|SetHealthbar)
  (CallFunction|SetStabilityBar))

(fn Kill
  (Actor|DestroyActor))

(fn CheckStun
  (if (<= (Variables|Default|GetStability) 0.0)
    (Variables|Default|SetIsStunned true)
    (AI|Components|Blackboard|SetValueasBool (Variables|Default|GetBlackboard) (Utilities|Name|MakeLiteralName "IsStunned") true)))

(fn CheckGrab
  (if (<= (/ (Variables|Default|GetHealth) (Variables|Default|GetMaxHealth)) (Variables|Default|GetGrabThreshhold))
    (Variables|Default|SetCanBeGrabbed true)
    (Class|ProgressBar|SetFillColorandOpacity (Variables|/Game/Blueprints/Enemies/EnemyBars.EnemyBars_C|GetHPBar (Variables|Default|GetBars)) "(R=0.863157,G=0.205079,B=0.045186,A=1.000000)")))

(fn SpawnHitVfx
  (bind _returnvalue (Transformation|GetActorLocation))
  (bind _capsulecomponent (Variables|Default|GetCapsuleComponent))
  (bind (_outradius _outhalfheight) (Components|Capsule|GetScaledCapsuleSize _capsulecomponent))
  (if (Utilities|IsValid self)
    (Game|SpawnActorfromClass "/Game/Blueprints/VFX/HitVfx.HitVfx_C" (Math|Transform|MakeTransform (Math|Vector|MakeVector (Math|Random|RandomFloatinRange (- (.x _returnvalue) _outradius) (+ (.x _returnvalue) _outradius)) 0.2 (Math|Random|RandomFloatinRange (- (.z _returnvalue) _outhalfheight) (+ (.z _returnvalue) _outhalfheight))) "0, 0, 0" (Variables|Default|GetHitVfxScale)) "AlwaysSpawn" self 0)))