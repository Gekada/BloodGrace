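; Green slime enemy Blueprint, a child class that takes nearly all of its behavior from its parent.
; On BeginPlay it runs the parent logic and then calls SetBars.
; Overlap, tick, damage, stability restore, construction and knockback damage overrides only forward to the parent implementations.
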(event EventBeginPlay
  (|CallParentFunction)
  (CallFunction|SetBars))

(event Collision|EventActorBeginOverlap
  (params (OtherActor :type Actor%20Object%20Reference))
  (|CallParentFunction OtherActor))

(event EventTick
  (params (DeltaSeconds :type Float%20%28single-precision%29))
  (|CallParentFunction DeltaSeconds))

(event EventOnStabilityRestore
  (|CallParentFunction))

(event Game|Damage|EventAnyDamage
  (params (Damage :type Float%20%28single-precision%29) (DamageType :type Damage%20Type%20Object%20Reference) (InstigatedBy :type Controller%20Object%20Reference) (DamageCauser :type Actor%20Object%20Reference))
  (|CallParentFunction Damage DamageType InstigatedBy DamageCauser))

(event EventOnDamageTaken
  (params (Damage :type Float%20%28double-precision%29) (Causer :type Actor%20Object%20Reference%20%28by%20ref%29))
  (|CallParentFunction Damage Causer))

(fn ConstructionScript
  (|CallParentFunction))

(fn ApplyDamagewithKnockback
  (params (Damage :type Float%20%28double-precision%29) (Dealer :type Actor%20Object%20Reference) (Knockback :type Vector :default "0, 0, 0"))
  (|CallParentFunction Damage Dealer Knockback))