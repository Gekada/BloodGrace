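; SpellKit is a component on the main hero character that provides a kit of three spell slots with cast and stop-cast events.
; On BeginPlay it caches its owner as MainHeroChar.
; Each cast, if movement is not blocked, blocks it and jumps the animation to the Spells node, with identical logic across slots, and each stop event unblocks movement.
; UpdateGUI applies the three spell icons and kit image to the HUD.
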(event Custom|CastFirst
  (bind _owner (Variables|Default|GetOwner))
  (if (not (Variables|/Game/Blueprints/MainHero/MainHeroChar.MainHeroChar_C|GetMovementBlocked _owner))
    (Variables|/Game/Blueprints/MainHero/MainHeroChar.MainHeroChar_C|SetMovementBlocked _owner true)
    (Class|PaperZDAnimInstance|JumptoNode (Variables|/Script/PaperZD.PaperZDAnimationComponent|GetAnimInstance (Variables|/Script/PaperZD.PaperZDCharacter|GetAnimationComponent _owner)) "Spells" "None")))

(event Custom|CastSecond
  (bind _owner (Variables|Default|GetOwner))
  (if (not (Variables|/Game/Blueprints/MainHero/MainHeroChar.MainHeroChar_C|GetMovementBlocked _owner))
    (Variables|/Game/Blueprints/MainHero/MainHeroChar.MainHeroChar_C|SetMovementBlocked _owner true)
    (Class|PaperZDAnimInstance|JumptoNode (Variables|/Script/PaperZD.PaperZDAnimationComponent|GetAnimInstance (Variables|/Script/PaperZD.PaperZDCharacter|GetAnimationComponent _owner)) "Spells" "None")))

(event Custom|CastThird
  (bind _owner (Variables|Default|GetOwner))
  (if (not (Variables|/Game/Blueprints/MainHero/MainHeroChar.MainHeroChar_C|GetMovementBlocked _owner))
    (Variables|/Game/Blueprints/MainHero/MainHeroChar.MainHeroChar_C|SetMovementBlocked _owner true)
    (Class|PaperZDAnimInstance|JumptoNode (Variables|/Script/PaperZD.PaperZDAnimationComponent|GetAnimInstance (Variables|/Script/PaperZD.PaperZDCharacter|GetAnimationComponent _owner)) "Spells" "None")))

(event Custom|StopCastFirst
  (Variables|/Game/Blueprints/MainHero/MainHeroChar.MainHeroChar_C|SetMovementBlocked (Variables|Default|GetOwner) false))

(event Custom|StopCastSecond
  (Variables|/Game/Blueprints/MainHero/MainHeroChar.MainHeroChar_C|SetMovementBlocked (Variables|Default|GetOwner) false))

(event Custom|StopCastThird
  (Variables|/Game/Blueprints/MainHero/MainHeroChar.MainHeroChar_C|SetMovementBlocked (Variables|Default|GetOwner) false))

(event EventBeginPlay
  (bind _asmain_hero_char (Utilities|Casting|CastToMainHeroChar (Components|GetOwner)))
  (Variables|Default|SetOwner _asmain_hero_char))

(fn UpdateGUI
  (bind _gui (Variables|Default|GetGUI))
  (Class|Image|SetBrush (Variables|/Game/UI/Blueprints/MainCharacterGUI.MainCharacterGUI_C|GetSkill1 _gui) (Variables|Default|GetFirstSpellImage))
  (Class|Image|SetBrush (Variables|/Game/UI/Blueprints/MainCharacterGUI.MainCharacterGUI_C|GetSkill2 _gui) (Variables|Default|GetSecondSpellImage))
  (Class|Image|SetBrush (Variables|/Game/UI/Blueprints/MainCharacterGUI.MainCharacterGUI_C|GetSkill3 _gui) (Variables|Default|GetThirdSpellImage))
  (Class|Image|SetBrush (Variables|/Game/UI/Blueprints/MainCharacterGUI.MainCharacterGUI_C|GetSkillKit _gui) (Variables|Default|GetKitImage)))